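; BP_BonusBall is a brick-breaker bonus brick that releases extra balls when it pops.
; Its OnPop function spawns six BP_otherBall actors, each at the location and rotation of one of six Arrow components, then destroys the brick.
; The construction script defers to the parent class, and the event graph holds only disabled placeholder events.
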(fn `OnPop`
  (bind (_returnvalue_location _returnvalue_rotation) (`KismetMathLibrary.BreakTransform` (`SceneComponent.K2_GetComponentToWorld` (`self.Arrow5`))))
  (bind (_returnvalue_location_2 _returnvalue_rotation_2) (`KismetMathLibrary.BreakTransform` (`SceneComponent.K2_GetComponentToWorld` (`self.Arrow3`))))
  (bind (_returnvalue_location_3 _returnvalue_rotation_3) (`KismetMathLibrary.BreakTransform` (`SceneComponent.K2_GetComponentToWorld` (`self.Arrow4`))))
  (bind (_returnvalue_location_4 _returnvalue_rotation_4) (`KismetMathLibrary.BreakTransform` (`SceneComponent.K2_GetComponentToWorld` (`self.Arrow`))))
  (bind (_returnvalue_location_5 _returnvalue_rotation_5) (`KismetMathLibrary.BreakTransform` (`SceneComponent.K2_GetComponentToWorld` (`self.Arrow1`))))
  (bind (_returnvalue_location_6 _returnvalue_rotation_6) (`KismetMathLibrary.BreakTransform` (`SceneComponent.K2_GetComponentToWorld` (`self.Arrow2`))))
  (`|SpawnActorFromClass` "/Game/BrickBreaker/Blueprints/BP_otherBall.BP_otherBall_C" (`KismetMathLibrary.MakeTransform` _returnvalue_location_4 _returnvalue_rotation_4) "Undefined" "MultiplyWithRoot" null null)
  (`|SpawnActorFromClass` "/Game/BrickBreaker/Blueprints/BP_otherBall.BP_otherBall_C" (`KismetMathLibrary.MakeTransform` _returnvalue_location_5 _returnvalue_rotation_5) "Undefined" "MultiplyWithRoot" null null)
  (`|SpawnActorFromClass` "/Game/BrickBreaker/Blueprints/BP_otherBall.BP_otherBall_C" (`KismetMathLibrary.MakeTransform` _returnvalue_location_6 _returnvalue_rotation_6) "Undefined" "MultiplyWithRoot" null null)
  (`|SpawnActorFromClass` "/Game/BrickBreaker/Blueprints/BP_otherBall.BP_otherBall_C" (`KismetMathLibrary.MakeTransform` _returnvalue_location_2 _returnvalue_rotation_2) "Undefined" "MultiplyWithRoot" null null)
  (`|SpawnActorFromClass` "/Game/BrickBreaker/Blueprints/BP_otherBall.BP_otherBall_C" (`KismetMathLibrary.MakeTransform` _returnvalue_location_3 _returnvalue_rotation_3) "Undefined" "MultiplyWithRoot" null null)
  (`|SpawnActorFromClass` "/Game/BrickBreaker/Blueprints/BP_otherBall.BP_otherBall_C" (`KismetMathLibrary.MakeTransform` _returnvalue_location _returnvalue_rotation) "Undefined" "MultiplyWithRoot" null null)
  (`self.K2_DestroyActor`))

(fn `UserConstructionScript`
  (`parent.UserConstructionScript`))