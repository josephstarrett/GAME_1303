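; BP_Multihit is a brick for the brick breaker game that takes several ball hits before it pops.
; Its OnHit increments a hit index and applies that entry of MaterialList to the SMBrick mesh, so each hit changes its look.
; Once the index runs past the end of the list it calls OnPop, so the material list's length sets the brick's durability.
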(fn `OnHit`
  (params (Ball :type "/Game/BrickBreaker/Blueprints/BP_Ball Object Reference"))
  (bind _result (`/Engine/EditorBlueprintResources/StandardMacros.IncrementInt` (`self.currentHit \\ Material Index`))
    (:`  `
      (if (>= _result (`KismetArrayLibrary.Array_Length` (`self.Material List`)))
        (`self.OnPop`)
        (else
          (`PrimitiveComponent.SetMaterial` (`self.SM_Brick`) 0 (`|GetArrayItem` (`self.Material List`) (`self.currentHit \\ Material Index`))))))))

(fn `UserConstructionScript`
  (`parent.UserConstructionScript`))