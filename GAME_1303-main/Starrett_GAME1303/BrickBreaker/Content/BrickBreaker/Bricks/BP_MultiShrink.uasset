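; BP_MultiShrink is a brick for the BrickBreaker game that takes multiple ball hits to pop.
; Each OnHit advances a hit index and sets the brick mesh to that entry in MaterialList.
; When the index runs past the list it calls OnPop, which only defers to the parent, so the material count sets durability.
; No shrink logic appears in this Blueprint itself.
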(fn `OnHit`
  (params (Ball :type "/Game/BrickBreaker/Blueprints/BP_Ball Object Reference"))
  (bind _result (`/Engine/EditorBlueprintResources/StandardMacros.IncrementInt` (`self.Hits / Material Index`))
    (:`  `
      (if (>= _result (`KismetArrayLibrary.Array_Length` (`self.MaterialList`)))
        (`self.OnPop`)
        (else
          (`PrimitiveComponent.SetMaterial` (`self.SM_Brick`) 0 (`|GetArrayItem` (`self.MaterialList`) (`self.Hits / Material Index`))))))))

(fn `OnPop`
  (`parent.OnPop`))

(fn `UserConstructionScript`
  (`parent.UserConstructionScript`))