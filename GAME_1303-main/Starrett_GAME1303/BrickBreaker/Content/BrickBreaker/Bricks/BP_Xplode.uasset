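; BP_Xplode is a Brick Breaker brick that shrinks away and removes itself when popped.
; OnPop disables collision on the collision component and mesh, then starts the shrink timer.
; Tick counts the timer down, scaling the mesh linearly from its BeginPlay size, and destroys the actor once the removal threshold is reached.
; Despite the name, no explosion logic appears here; construction defers to the parent class.
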(event `self.ReceiveBeginPlay`
  (set `self.StartingSize` (`SceneComponent.RelativeScale3D` (`self.SM_Brick`))))

(event `self.ReceiveTick`
  (params (DeltaSeconds :type "Float (single-precision)"))
  (if (`self.IsShrinking`)
    (bind _output_get (set `self.ShrinkTimer` (- (`self.ShrinkTimer`) DeltaSeconds)))
    (if (<= _output_get (`self.RemoveAtTime`))
      (`self.K2_DestroyActor`)
      (else
        (`SceneComponent.SetRelativeScale3D` (`self.SM_Brick`) (* (/ (`self.ShrinkTimer`) (`self.ShrinkTime`)) (`self.StartingSize`)))))))

(fn `OnPop`
  (set `self.IsShrinking` true)
  (`PrimitiveComponent.SetCollisionEnabled` (`self.COL_Brick`) "NoCollision")
  (`PrimitiveComponent.SetCollisionEnabled` (`self.SM_Brick`) "NoCollision")
  (set `self.ShrinkTimer` (`self.ShrinkTime`)))

(fn `UserConstructionScript`
  (`parent.UserConstructionScript`))