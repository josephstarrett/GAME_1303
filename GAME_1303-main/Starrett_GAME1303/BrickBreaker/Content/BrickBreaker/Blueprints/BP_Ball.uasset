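; BP_Ball is the brick breaker ball, moved by a ProjectileMovement component.
; On BeginPlay it can set a start velocity from InitialSpeed, though the random Y range has equal bounds, so the direction is fixed.
; Each hit on its mesh calls CheckZ, prints the other actor's name and plays a boing sound.
; CheckZ keeps play planar by resetting any nonzero Z position and its vertical velocity to zero.
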(event `self.ReceiveTick`
  (params (DeltaSeconds :type "Float (single-precision)")))

(event `self.ReceiveBeginPlay`
  (if (`self.HasRandomStartVelocity`)
    (`self.Set Random Start Velocity`)))

(event `self.SM_Ball.OnComponentHit`
  (params (HitComponent :type "PrimitiveComponent Object Reference") (OtherActor :type "Actor Object Reference") (OtherComp :type "PrimitiveComponent Object Reference") (NormalImpulse :type "Vector Structure") (Hit :type "HitResult Structure (by ref)"))
  (`self.Check Z`)
  (`KismetSystemLibrary.PrintString` (`KismetSystemLibrary.GetDisplayName` OtherActor))
  (`GameplayStatics.PlaySound2D` "/Game/BrickBreaker/Audio/ac_Boing.ac_Boing" 1.0 1.0 0.0 null null))

(fn `Check Z`
  (bind _returnvalue (`self.GetTransform`))
  (bind _projectilemovement (`self.ProjectileMovement`))
  (bind (_velocity_x _velocity_y) (`KismetMathLibrary.BreakVector` (`MovementComponent.Velocity` _projectilemovement)))
  (if (!= (.z (.location _returnvalue)) 0.0)
    (`self.K2_SetActorLocation` (`KismetMathLibrary.MakeVector` (.x (.location _returnvalue)) (.y (.location _returnvalue))))
    (set `MovementComponent.Velocity` (`KismetMathLibrary.MakeVector` _velocity_x _velocity_y) _projectilemovement)))

(fn `Set Random Start Velocity`
  (set `MovementComponent.Velocity` (* (`KismetMathLibrary.MakeVector` 1.0 (`KismetMathLibrary.RandomFloatInRange` -0.3 -0.3)) (`ProjectileMovementComponent.InitialSpeed` (`self.ProjectileMovement`))) (`self.ProjectileMovement`)))

(fn `UserConstructionScript`)