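; Lab07 HUD Blueprint that sets up the main menu and About panel UI at game start.
; On BeginPlay it shows the mouse cursor, then creates both widgets and adds only the main menu to the viewport.
; It stores each widget in the other's reference variable, so the menu and About panel can reach one another directly.
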(event `self.ReceiveBeginPlay`
  (set `PlayerController.bShowMouseCursor` true (`GameplayStatics.GetPlayerController` 0))
  (bind _returnvalue (`|CreateWidget` "/Game/Lab07/BPW_Lab07_MainMenu.BPW_Lab07_MainMenu_C"))
  (bind _output_get (set `self.MainMenuWidget(inHUD) ` _returnvalue))
  (`UserWidget.AddToViewport` _output_get 0)
  (bind _returnvalue_2 (`|CreateWidget` "/Game/Lab07/BPW_Lab07_AboutPanel.BPW_Lab07_AboutPanel_C"))
  (set `self.AboutPanelWidget(inHUD)` _returnvalue_2)
  (set `/Game/Lab07/BPW_Lab07_MainMenu.AboutPanel (inMainMenuWidget` (`self.AboutPanelWidget(inHUD)`) (`self.MainMenuWidget(inHUD) `))
  (set `/Game/Lab07/BPW_Lab07_AboutPanel.MainMenu (inAboutPanelWidget)` (`self.MainMenuWidget(inHUD) `) (`self.AboutPanelWidget(inHUD)`)))

(fn `UserConstructionScript`)