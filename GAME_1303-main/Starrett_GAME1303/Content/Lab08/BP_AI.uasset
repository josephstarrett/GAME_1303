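; BP_AI is a Lab08 enemy that chases the player's pawn with AIMoveTo, starting at BeginPlay.
; Each successful move waits briefly, plays a white-noise sound at the AI's location and restarts the chase.
; A failed move has no retry of its own, but VisionTick restarts the chase when a BP_Lab08_PAWN overlaps its Box; no caller for VisionTick appears here.
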(event `self.ReceiveBeginPlay`
  (`self.MoveToPlayer`))

(event `MoveToPlayer`
  (`|AIMoveTo` self (0.0 0.0 0.0) (`Controller.K2_GetPawn` (`GameplayStatics.GetPlayerController` 0)) (`self.WithinRange`) true
    (:`OnSuccess`
      (`KismetSystemLibrary.Delay` 0.2)
      (`GameplayStatics.PlaySoundAtLocation` "/Engine/EngineSounds/WhiteNoise.WhiteNoise" (`self.K2_GetActorLocation`) (struct) 1.0 1.0 0.0 null null null null)
      (`self.MoveToPlayer`))))

(event `VisionTick`
  (if (> (`KismetArrayLibrary.Array_Length` (`PrimitiveComponent.GetOverlappingActors` (`self.Box`) "/Game/Lab08/BP_Lab08_PAWN.BP_Lab08_PAWN_C")) 0)
    (`self.MoveToPlayer`)))

(fn `UserConstructionScript`)