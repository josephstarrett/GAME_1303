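; BP_ItGoesBoom is a usable actor that explodes when used.
; Its OnUse override calls the parent implementation, spawns the P_Explosion emitter and Explosion_Cue sound at the actor's location, then destroys the actor.
; The effect is purely audiovisual, with no damage or physics logic in this Blueprint, and the event graph holds only disabled default events.
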(fn `OnUse`
  (bind (_returnvalue_location _returnvalue_rotation) (`KismetMathLibrary.BreakTransform` (`self.GetTransform`)))
  (`parent.OnUse`)
  (`GameplayStatics.SpawnEmitterAtLocation` "/Game/StarterContent/Particles/P_Explosion.P_Explosion" _returnvalue_location _returnvalue_rotation)
  (`GameplayStatics.SpawnSoundAtLocation` "/Game/StarterContent/Audio/Explosion_Cue.Explosion_Cue" (`self.K2_GetActorLocation`) (struct) 1.0 1.0 0.0 null null)
  (`self.K2_DestroyActor`))

(fn `UserConstructionScript`
  (`parent.UserConstructionScript`))