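; BP_Elevator is a usable lift that travels to a target position when used, then returns automatically.
; OnUse starts a timeline whose percent drives MoveLift, lerping the Model's relative location from its BeginPlay position to that of the Phatom component.
; When the timeline finishes, it waits a configurable delay and reverses, with the HasBeenActivated flag keeping the reverse run from triggering another return.
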(event `self.ReceiveBeginPlay`
  (set `self.LiftStartingPosition` (`SceneComponent.RelativeLocation` (`self.Model`))))

(event `Start Lift`
  (set `self.HasBeenActivated` true)
  (bind (_direction _percent) (`Timeline|Timeline` :!label _label)
    (:`Update`
      (`self.MoveLift` _percent))
    (:`Finished`
      (if (`self.HasBeenActivated`)
        (set `self.HasBeenActivated` false)
        (`KismetSystemLibrary.Delay` (`self.ReturnDealy`))
        (`self.Return Lift`)))))

(event `Return Lift`
  (goto _label :!via `Reverse`))

(fn `MoveLift`
  (params (Percent :type "Float (double-precision)"))
  (`SceneComponent.K2_SetRelativeLocation` (`self.Model`) (`KismetMathLibrary.VLerp` (`self.LiftStartingPosition`) (`SceneComponent.RelativeLocation` (`self.Phatom`)) Percent) false false))

(fn `OnUse`
  (`parent.OnUse`)
  (`self.Start Lift`))

(fn `UserConstructionScript`
  (`parent.UserConstructionScript`))