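; BP_Collectible is a pickup actor for the collection minigame.
; When a BP_CollectionPawn overlaps its collision component, it registers itself with BP_CollectionGameMode through AddCollectedItem, then calls OnTaken.
; OnTaken plays an explosion sound and spawns an emitter at the actor's location, then destroys the actor.
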(event `self.Collision.OnComponentBeginOverlap`
  (params (OverlappedComponent :type "PrimitiveComponent Object Reference") (OtherActor :type "Actor Object Reference") (OtherComp :type "PrimitiveComponent Object Reference") (OtherBodyIndex :type Integer) (bFromSweep :type Boolean) (SweepResult :type "HitResult Structure (by ref)"))
  (cast `/Game/CollectionMiniGame/BP_CollectionPawn` OtherActor)
  (bind _asbp_collection_game_mode (cast `/Game/CollectionMiniGame/HUD/BP_CollectionGameMode` (`GameplayStatics.GetGameMode`)))
  (`/Game/CollectionMiniGame/HUD/BP_CollectionGameMode.AddCollectedItem` _asbp_collection_game_mode self)
  (`self.OnTaken`))

(fn `OnTaken`
  (`GameplayStatics.PlaySoundAtLocation` "/Game/StarterContent/Audio/Explosion_Cue.Explosion_Cue" (`self.K2_GetActorLocation`) (struct) 1.0 1.0 0.0 null null null null)
  (`GameplayStatics.SpawnEmitterAtLocation` null (`self.K2_GetActorLocation`) (`self.K2_GetActorRotation`))
  (`self.K2_DestroyActor`))

(fn `UserConstructionScript`)