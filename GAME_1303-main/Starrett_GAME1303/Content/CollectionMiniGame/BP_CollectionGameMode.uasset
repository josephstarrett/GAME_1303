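; Game mode for a timed collection minigame that tracks application state, remaining time, score and items collected.
; StartGame, also called by RestartGame, resets those values and starts a looping one-second Clock timer that counts down, then switches state and stops itself at zero.
; AddCollectedItem adds an item's awarded score and bumps the count, while AddGameTime extends the remaining time.
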(event `self.ReceiveBeginPlay`)

(event `Restart Game`
  (`self.StartGame`))

(fn `AddCollectedItem`
  (params (CollectedItem :type "/Game/CollectionMiniGame/BP_Collectible Object Reference"))
  (locals (NewLocalVar :type Integer :default 0))
  (set `self.GameScore` (+ (`/Game/CollectionMiniGame/BP_Collectible.ScoreAwarded` CollectedItem) (`self.GameScore`)))
  (`/Engine/EditorBlueprintResources/StandardMacros.IncrementInt` (`self.ItemsCollected`)))

(fn `AddGameTime`
  (params (AddedTime :type Integer))
  (set `self.TImeRemaining` (+ AddedTime (`self.TImeRemaining`))))

(fn `Clock`
  (bind _result (`/Engine/EditorBlueprintResources/StandardMacros.DecrementInt` (`self.TImeRemaining`))
    (:`  `
      (if (<= _result 0)
        (set `self.Application State` "NewEnumerator2")
        (`KismetSystemLibrary.K2_ClearTimer` null "Clock")))))

(fn `UserConstructionScript`)