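; BP_CollectionHUD is the HUD for the collection minigame, showing time remaining, score and items collected.
; It caches a reference to BP_CollectionGameMode on BeginPlay and reads its values each frame in DrawHUD.
; DrawHUD switches on the game mode's GameOver flag between the colored stats readout and a large GAME OVER message, both drawn with canvas DrawText rather than UMG widgets.
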(event `self.ReceiveBeginPlay`
  (bind _asbp_collection_game_mode (cast `/Game/CollectionMiniGame/BP_CollectionGameMode` (`GameplayStatics.GetGameMode`)))
  (set `self.GameMode` _asbp_collection_game_mode))

(event `self.ReceiveDrawHUD`
  (params (SizeX :type Integer) (SizeY :type Integer))
  (if (`/Game/CollectionMiniGame/BP_CollectionGameMode.GameOver` (`self.GameMode`))
    (`self.DrawGameOverHud`)
    (else
      (`self.DrawGameHUD`))))

(fn `DrawGameHUD`
  (`self.DrawText` (`KismetStringLibrary.Concat_StrStr` "Time: " (`KismetStringLibrary.Conv_IntToString` (`/Game/CollectionMiniGame/BP_CollectionGameMode.TImeRemaining` (`self.GameMode`)))) (struct :`R` 0.79 :`A` 1.0) 30.0 50.0 null 2.0)
  (`self.DrawText` (`KismetStringLibrary.Concat_StrStr` "Score: " (`KismetStringLibrary.Conv_IntToString` (`/Game/CollectionMiniGame/BP_CollectionGameMode.GameScore` (`self.GameMode`)))) (struct :`R` 1.0 :`G` 0.937268 :`B` 0.069704 :`A` 1.0) 30.0 75.0 null 2.0)
  (`self.DrawText` (`KismetStringLibrary.Concat_StrStr` "items: " (`KismetStringLibrary.Conv_IntToString` (`/Game/CollectionMiniGame/BP_CollectionGameMode.ItemsCollected` (`self.GameMode`)))) (struct :`G` 1.0 :`B` 0.075343 :`A` 1.0) 30.0 100.0 null 2.0))

(fn `DrawGameOverHud`
  (`self.DrawText` "GAME OVER!" (struct :`R` 0.86 :`A` 1.0) 30.0 50.0 null 4.02))

(fn `UserConstructionScript`)