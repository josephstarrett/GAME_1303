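; HUD class for the collection minigame that switches between main menu, gameplay and game over screens.
; BeginPlay caches BP_CollectionGameMode, then creates all three widgets and adds them to the viewport.
; Every DrawHUD call polls the game mode's ApplicationState, shows the matching widget, hides the other two and toggles the mouse cursor, which appears only outside gameplay.
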(event `self.ReceiveBeginPlay`
  (bind _asbp_collection_game_mode (cast `/Game/CollectionMiniGame/HUD/BP_CollectionGameMode` (`GameplayStatics.GetGameMode`)))
  (set `self.GameMode` _asbp_collection_game_mode)
  (bind _returnvalue (`|CreateWidget` "/Game/CollectionMiniGame/HUD/BPW_MainMenu.BPW_MainMenu_C"))
  (bind _output_get (set `self.MainMenuWidget` _returnvalue))
  (`UserWidget.AddToViewport` _output_get 0)
  (bind _returnvalue_2 (`|CreateWidget` "/Game/CollectionMiniGame/HUD/BPW_GameHud.BPW_GameHud_C"))
  (bind _output_get_2 (set `self.GameHudWidget` _returnvalue_2))
  (`UserWidget.AddToViewport` _output_get_2 0)
  (bind _returnvalue_3 (`|CreateWidget` "/Game/CollectionMiniGame/HUD/BPW_GameOver.BPW_GameOver_C"))
  (bind _output_get_3 (set `self.GameOverWidget` _returnvalue_3))
  (`UserWidget.AddToViewport` _output_get_3 0))

(event `self.ReceiveDrawHUD`
  (params (SizeX :type Integer) (SizeY :type Integer))
  (switch `/Game/CollectionMiniGame/HUD/AppStateEnum` (`/Game/CollectionMiniGame/HUD/BP_CollectionGameMode.Application State` (`self.GameMode`))
    (:`NewEnumerator0`
      (`self.DrawMainMenu`))
    (:`NewEnumerator1`
      (`self.DrawGameHUD`))
    (:`NewEnumerator2`
      (`self.DrawGameOverHud`))))

(fn `DrawGameHUD`
  (set `PlayerController.bShowMouseCursor` false (`GameplayStatics.GetPlayerController` 0))
  (`Widget.SetVisibility` (`self.MainMenuWidget`) "Hidden")
  (`Widget.SetVisibility` (`self.GameHudWidget`) "Visible")
  (`Widget.SetVisibility` (`self.GameOverWidget`) "Hidden"))

(fn `DrawGameOverHud`
  (set `PlayerController.bShowMouseCursor` true (`GameplayStatics.GetPlayerController` 0))
  (`Widget.SetVisibility` (`self.MainMenuWidget`) "Hidden")
  (`Widget.SetVisibility` (`self.GameHudWidget`) "Hidden")
  (`Widget.SetVisibility` (`self.GameOverWidget`) "Visible"))

(fn `DrawMainMenu`
  (set `PlayerController.bShowMouseCursor` true (`GameplayStatics.GetPlayerController` 0))
  (`Widget.SetVisibility` (`self.MainMenuWidget`) "Visible")
  (`Widget.SetVisibility` (`self.GameHudWidget`) "Hidden")
  (`Widget.SetVisibility` (`self.GameOverWidget`) "Hidden"))

(fn `UserConstructionScript`)