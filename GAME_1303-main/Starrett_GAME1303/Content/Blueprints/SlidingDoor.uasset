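; Sliding double door that opens when something overlaps its collision trigger and closes when the overlap ends.
; BeginPlay caches both doors' relative start locations, with the DoorAStart and DoorBStart names swapped relative to their components but used consistently.
; A Timeline plays or reverses on overlap, feeding its Percentage to a shared SlideDoor function that offsets the doors along local Y in opposite directions by SlideAmount.
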(event `self.ReceiveBeginPlay`
  (set `self.DoorAStart` (`SceneComponent.RelativeLocation` (`self.DoorB`)))
  (set `self.DoorBStart` (`SceneComponent.RelativeLocation` (`self.DoorA`))))

(event `self.Collision Trigger.OnComponentBeginOverlap`
  (params (OverlappedComponent :type "PrimitiveComponent Object Reference") (OtherActor :type "Actor Object Reference") (OtherComp :type "PrimitiveComponent Object Reference") (OtherBodyIndex :type Integer) (bFromSweep :type Boolean) (SweepResult :type "HitResult Structure (by ref)"))
  (bind (_direction _percentage) (`Timeline|Timeline` :!label _label)
    (:`Update`
      (`self.SlideDoor` (`self.DoorB`) (`self.DoorAStart`) 1.0 _percentage)
      (`self.SlideDoor` (`self.DoorA`) (`self.DoorBStart`) -1.0 _percentage))))

(event `self.Collision Trigger.OnComponentEndOverlap`
  (params (OverlappedComponent :type "PrimitiveComponent Object Reference") (OtherActor :type "Actor Object Reference") (OtherComp :type "PrimitiveComponent Object Reference") (OtherBodyIndex :type Integer))
  (goto _label :!via `Reverse`))

(fn `SlideDoor`
  (params (`The Door` :type "StaticMeshComponent Object Reference") (`Start Location` :type "Vector Structure") (Direction :type "Float (double-precision)") (Percentage :type "Float (double-precision)"))
  (`SceneComponent.K2_SetRelativeLocation` `The Door` (`KismetMathLibrary.MakeVector` `Start Location_X` (+ `Start Location_Y` (* Direction (* Percentage (`self.SlideAmount`)))) `Start Location_Z`) false false))

(fn `UserConstructionScript`)